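; Double door actor that lets the player open a left or right door, apparently through a vote, while inside its trigger box.
; Box overlap toggles the voting-time widget and flags on the player controller and character, clearing vote counts on exit.
; While overlapped, Tick polls the controller's LeftDoor and RightDoor flags, playing a timeline that yaws the matching hinge and resets that flag, with left taking priority.
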(event OnComponentBeginOverlap(Box)
  (params (OverlappedComponent :type Primitive%20Component%20Object%20Reference) (OtherActor :type Actor%20Object%20Reference) (OtherComp :type Primitive%20Component%20Object%20Reference) (OtherBodyIndex :type Integer) (bFromSweep :type Boolean) (SweepResult :type Hit%20Result%20Structure%20%28by%20ref%29))
  (bind _returnvalue (UserInterface|CreateWidget "/Game/Assets/Blueprints/WB_VotingTimeMessage.WB_VotingTimeMessage_C"))
  (UserInterface|Viewport|AddtoViewport _returnvalue 0)
  (Variables|Default|Setoverlapped true)
  (bind _asbp_third_person_game_mode (Utilities|Casting|CastToBP_ThirdPersonGameMode (Game|GetGameMode)))
  (Variables|/Game/ThirdPerson/Blueprints/BP_ThirdPersonGameMode.BP_ThirdPersonGameMode_C|SetDoubleDoorOverlap _asbp_third_person_game_mode 0)
  (Development|PrintString "DoubleDoor")
  (bind _asbp_game_pc (Utilities|Casting|CastToBP_GamePC (Game|GetPlayerController 0)))
  (Variables|/Game/Assets/Blueprints/Chat/BP_GamePC.BP_GamePC_C|SetGameBeginDoorOpen _asbp_game_pc true)
  (bind _asbp_third_person_character (Utilities|Casting|CastToBP_ThirdPersonCharacter (Game|GetPlayerCharacter 0)))
  (Variables|/Game/ThirdPerson/Blueprints/BP_ThirdPersonCharacter.BP_ThirdPersonCharacter_C|SetisOverlapping _asbp_third_person_character true)
  (Variables|Default|SetIsLeftAndRightDoor true))

(event OnComponentEndOverlap(Box)
  (params (OverlappedComponent :type Primitive%20Component%20Object%20Reference) (OtherActor :type Actor%20Object%20Reference) (OtherComp :type Primitive%20Component%20Object%20Reference) (OtherBodyIndex :type Integer))
  (Widget|RemovefromParent (stale OnComponentBeginOverlap(Box) _returnvalue))
  (Variables|Default|Setoverlapped false)
  (bind _asbp_game_pc (Utilities|Casting|CastToBP_GamePC (Game|GetPlayerController 0)))
  (Variables|/Game/Assets/Blueprints/Chat/BP_GamePC.BP_GamePC_C|SetGameBeginDoorOpen _asbp_game_pc false)
  (bind _asbp_third_person_character (Utilities|Casting|CastToBP_ThirdPersonCharacter (Game|GetPlayerCharacter 0)))
  (Variables|/Game/ThirdPerson/Blueprints/BP_ThirdPersonCharacter.BP_ThirdPersonCharacter_C|SetisOverlapping _asbp_third_person_character false)
  (Variables|Default|SetIsLeftAndRightDoor false)
  (Variables|/Game/ThirdPerson/Blueprints/BP_ThirdPersonCharacter.BP_ThirdPersonCharacter_C|SetVotes%20Forward (stale OnComponentBeginOverlap(Box) _asbp_third_person_character) 0.0)
  (Variables|/Game/ThirdPerson/Blueprints/BP_ThirdPersonCharacter.BP_ThirdPersonCharacter_C|SetVotes%20Right (stale OnComponentBeginOverlap(Box) _asbp_third_person_character) 0.0)
  (Variables|/Game/ThirdPerson/Blueprints/BP_ThirdPersonCharacter.BP_ThirdPersonCharacter_C|SetVotes%20Left (stale OnComponentBeginOverlap(Box) _asbp_third_person_character) 0.0))

(event EventBeginPlay)

(event Collision|EventActorBeginOverlap
  (params (OtherActor :type Actor%20Object%20Reference)))

(event EventTick
  (params (DeltaSeconds :type Float%20%28single-precision%29))
  (if (Variables|Default|Getoverlapped)
    (bind _asbp_game_pc (Utilities|Casting|CastToBP_GamePC (Game|GetPlayerController 0)))
    (if (Variables|/Game/Assets/Blueprints/Chat/BP_GamePC.BP_GamePC_C|GetLeftDoor _asbp_game_pc)
      (bind _newtrack_0 (Timeline|Timeline Play)
        (:Update
          (Transformation|SetRelativeRotation (Variables|Default|GetHingeLeft) (Math|Rotator|MakeRotator 0.0 0.0 _newtrack_0) false false)
          (bind _asbp_game_pc_2 (Utilities|Casting|CastToBP_GamePC (Game|GetPlayerController 0)))
          (Variables|/Game/Assets/Blueprints/Chat/BP_GamePC.BP_GamePC_C|SetLeftDoor _asbp_game_pc_2 false)))
      (elif (Variables|/Game/Assets/Blueprints/Chat/BP_GamePC.BP_GamePC_C|GetRightDoor _asbp_game_pc)
        (bind _newtrack_0_2 (Timeline|Timeline_0 Play)
          (:Update
            (Transformation|SetRelativeRotation (Variables|Default|GetHingeRight) (Math|Rotator|MakeRotator 0.0 0.0 _newtrack_0_2) false false)
            (bind _asbp_game_pc_3 (Utilities|Casting|CastToBP_GamePC (Game|GetPlayerController 0)))
            (Variables|/Game/Assets/Blueprints/Chat/BP_GamePC.BP_GamePC_C|SetRightDoor _asbp_game_pc_3 false)))))))

(fn ConstructionScript)