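; Player controller component that provides in-game text chat, creating and displaying the chat UI widget for the local controller on BeginPlay.
; Enter focuses the chat box and mouse wheel up scrolls it; the downward scroll call is unconnected.
; Messages go through a server event that loops over the GameState PlayerArray and calls each controller's chat component, whose owning-client event adds the message to the chat box.
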(event Custom|SendChatMessageOnServer
  (params (Message :type String))
  (for _array_element (Variables|/Script/Engine.GameStateBase|GetPlayerArray (Game|GetGameState))
    (CallFunction|AddChatMessageonOwningClient (Actor|GetComponentbyClass (Game|GetPlayerController _array_element) "AC_Chat_PC_C") Message)))

(event Custom|AddChatMessageOnOwningClient
  (params (Message :type String))
  (Default|AddChatMessage (Variables|Default|GetChatBoxRef) Message))

(event EventBeginPlay
  (if (Pawn|IsLocalController (.AsPlayer%20Controller (Utilities|Casting|CastToPlayerController (Components|GetOwner))))
    (bind _returnvalue (UserInterface|CreateWidget "/Game/Assets/Blueprints/Chat/WB_ChatUI.WB_ChatUI_C"))
    (bind _output_get (Variables|Default|SetChatUIRef _returnvalue))
    (UserInterface|Viewport|AddtoViewport _output_get 0)))

(event Input|KeyboardEvents|Enter
  (params (Key :type Key%20Structure :default "None"))
  (:Pressed
    (Default|FocusChat (Variables|Default|GetChatBoxRef))))

(event Input|MouseEvents|MouseWheelUp
  (params (Key :type Key%20Structure :default "None"))
  (:Pressed
    (Default|Scroll (Variables|Default|GetChatBoxRef) true)))

(event Input|MouseEvents|MouseWheelDown
  (params (Key :type Key%20Structure :default "None")))