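; BP_GamePC receives commands to open the left, right or forward door and records them as state flags.
; Each of the three custom events sets the flag for its door, then raises a shared DoorCommand flag if GameBeginDoorOpen is true.
; The Blueprint only sets these variables and moves no doors itself; BeginPlay, Tick and the construction script are empty.
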(event Custom|OpenLeftDoor
  (Variables|Default|SetLeftDoor true)
  (if (Variables|Default|GetGameBeginDoorOpen)
    (Variables|Default|SetDoorCommand true)))

(event Custom|OpenRightDoor
  (Variables|Default|SetRightDoor true)
  (if (Variables|Default|GetGameBeginDoorOpen)
    (Variables|Default|SetDoorCommand true)))

(event Custom|OpenForwardDoor
  (Variables|Default|SetForwardDoor true)
  (if (Variables|Default|GetGameBeginDoorOpen)
    (Variables|Default|SetDoorCommand true)))

(event EventBeginPlay)

(event EventTick
  (params (DeltaSeconds :type Float%20%28single-precision%29)))

(fn ConstructionScript)